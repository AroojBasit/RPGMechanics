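; Player stats component for BP_ThirdPersonCharacter that tracks health, stamina, XP and level.
; On BeginPlay it waits a tick, caches the owning character and pushes all values to its HUD widget.
; Increase and decrease functions cap gains at max, report depletion through a bool and refresh the matching HUD element.
; Reaching MaxXP levels up, which resets XP, raises the next threshold and plays level-up sounds.
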(event EventBeginPlay
  (Utilities|FlowControl|DelayUntilNextTick)
  (bind _asbp_third_person_character (Utilities|Casting|CastToBP_ThirdPersonCharacter (Components|GetOwner)))
  (Variables|Default|SetPlayerCharacter _asbp_third_person_character)
  (HUD|UpdateHUDHealth)
  (HUD|UpdateHUDStamina)
  (HUD|UpdateHUDXP)
  (HUD|UpdateHUDLevel))

(event EventTick
  (params (DeltaSeconds :type Float%20%28single-precision%29)))

(fn DecreaseHealth
  (params (Damage :type Float%20%28double-precision%29))
  (if (not (<= (Variables|Health|GetCurrentHealth) 0.0))
    (Variables|Health|SetCurrentHealth (- (Variables|Health|GetCurrentHealth) Damage))
    (HUD|UpdateHUDHealth)
    (if (<= (Variables|Health|GetCurrentHealth) 0.0)
      _
      (else
        (return false))))
  (return true))

(fn IncreaseHealth
  (params (Delta :type Float%20%28double-precision%29))
  (bind _output_get (Variables|Health|SetCurrentHealth (+ (Variables|Health|GetCurrentHealth) Delta)))
  (if (> _output_get (Variables|Health|GetMaxHealth))
    (Variables|Health|SetCurrentHealth (Variables|Health|GetMaxHealth)))
  (HUD|UpdateHUDHealth))

(fn IncreaseMaxHealth
  (params (Delta :type Float%20%28double-precision%29))
  (Variables|Health|SetMaxHealth (+ (Variables|Health|GetMaxHealth) Delta))
  (HUD|UpdateHUDHealth))

(fn DecreaseStamina
  (params (Delta :type Float%20%28double-precision%29))
  (if (not (<= (Variables|Stemina|GetCurrentStamina) 0.0))
    (Variables|Stemina|SetCurrentStamina (- (Variables|Stemina|GetCurrentStamina) Delta))
    (HUD|UpdateHUDStamina)
    (if (<= (Variables|Stemina|GetCurrentStamina) 0.0)
      _
      (else
        (return false))))
  (return true))

(fn IncreaseStamina
  (params (Delta :type Float%20%28double-precision%29))
  (bind _output_get (Variables|Stemina|SetCurrentStamina (+ (Variables|Stemina|GetCurrentStamina) Delta)))
  (if (> _output_get (Variables|Stemina|GetMaxStamina))
    (Variables|Stemina|SetCurrentStamina (Variables|Stemina|GetMaxStamina)))
  (HUD|UpdateHUDStamina))

(fn IncreaseMaxStamina
  (params (Delta :type Float%20%28double-precision%29))
  (Variables|Stemina|SetMaxStamina (+ (Variables|Stemina|GetMaxStamina) Delta))
  (HUD|UpdateHUDStamina))

(fn UpdateHUDHealth
  (bind _playercharacter (Variables|Default|GetPlayerCharacter))
  (bind _hud_widget (Variables|/Game/ThirdPerson/Blueprints/BP_ThirdPersonCharacter.BP_ThirdPersonCharacter_C|GetHUD_Widget _playercharacter))
  (Variables|/Script/UMG.TextBlock|SetText (Variables|/Game/UI/WB_HUD.WB_HUD_C|GetHealthText _hud_widget) (Utilities|Text|ToText(Float) (Variables|Health|GetCurrentHealth) "HalfToEven"))
  (Progress|SetPercent (Variables|/Game/UI/WB_HUD.WB_HUD_C|GetHealthBar _hud_widget) (/ (Variables|Health|GetCurrentHealth) (Variables|Health|GetMaxHealth))))

(fn UpdateHUDStamina
  (Progress|SetPercent (Variables|/Game/UI/WB_HUD.WB_HUD_C|GetStaminaBar (Variables|/Game/ThirdPerson/Blueprints/BP_ThirdPersonCharacter.BP_ThirdPersonCharacter_C|GetHUD_Widget (Variables|Default|GetPlayerCharacter))) (/ (Variables|Stemina|GetCurrentStamina) (Variables|Stemina|GetMaxStamina))))

(fn IncreaseXP
  (params (Delta :type Float%20%28double-precision%29))
  (bind _output_get (Variables|XP|SetXP (+ (Variables|XP|GetXP) Delta)))
  (if (>= _output_get (Variables|XP|GetMaxXP))
    (XP|IncreaseLevel 1))
  (HUD|UpdateHUDXP))

(fn IncreaseLevel
  (params (Delta :type Integer))
  (Variables|XP|SetLevel (+ (Variables|XP|GetLevel) Delta))
  (Variables|XP|SetMaxXP (+ (Variables|XP|GetMaxXP) 1.5e+02))
  (Variables|XP|SetXP 0.0)
  (HUD|UpdateHUDLevel)
  (Audio|PlaySound2D "/Game/Audio/UI/LevelUp1.LevelUp1" 1.0 1.0 0.0 0 0)
  (Audio|PlaySound2D "/Game/Audio/UI/LevelUp2.LevelUp2" 1.0 1.0 0.0 0 0))

(fn UpdateHUDXP
  (bind _playercharacter (Variables|Default|GetPlayerCharacter))
  (bind _hud_widget (Variables|/Game/ThirdPerson/Blueprints/BP_ThirdPersonCharacter.BP_ThirdPersonCharacter_C|GetHUD_Widget _playercharacter))
  (Variables|/Script/UMG.TextBlock|SetText (Variables|/Game/UI/WB_HUD.WB_HUD_C|GetXPText _hud_widget) (Utilities|Text|FormatText "{XP} / {MaxXP}" (Variables|XP|GetXP) (Variables|XP|GetMaxXP)))
  (Progress|SetPercent (Variables|/Game/UI/WB_HUD.WB_HUD_C|GetXPBar _hud_widget) (/ (Variables|XP|GetXP) (Variables|XP|GetMaxXP))))

(fn UpdateHUDLevel
  (Variables|/Script/UMG.TextBlock|SetText (Variables|/Game/UI/WB_HUD.WB_HUD_C|GetLevelText (Variables|/Game/ThirdPerson/Blueprints/BP_ThirdPersonCharacter.BP_ThirdPersonCharacter_C|GetHUD_Widget (Variables|Default|GetPlayerCharacter))) (Utilities|Text|ToText(Integer) (Variables|XP|GetLevel))))